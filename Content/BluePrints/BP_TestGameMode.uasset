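; BP_TestGameMode is a test game mode that spawns tracker bots at locations chosen by an EQS query.
; BeginPlay runs EQS_FindSpawnLocation in random-best-25% mode, binds its finished event, and prints "Query done" without waiting for completion.
; On success, it draws a debug sphere at each returned location and spawns BP_TrackerBot there, adjusting for collisions or skipping the spawn if still blocked.
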(event Custom|OnQueryFinishedEvent_Event_0
  (params (QueryInstance :type Env%20Query%20Instance%20Blueprint%20Wrapper%20Object%20Reference) (QueryStatus :type EEnvQueryStatus%20Enum :default "Processing"))
  (switch Utilities|FlowControl|Switch|SwitchonEEnvQueryStatus QueryStatus
    (:Success
      (Development|PrintString "Successful" true true "(R=0.000000,G=0.660000,B=1.000000,A=1.000000)" 1e+01)
      (bind _resultlocations (AI|EQS|GetQueryResultsasLocations QueryInstance))
      (for _array_element _resultlocations
        (Rendering|Debug|DrawDebugSphere _array_element 5e+01 12 "(R=1.000000,G=0.870406,B=0.000000,A=1.000000)" 1e+01 1.0)
        (Game|SpawnActorfromClass "/Game/TrackerBot/BP_TrackerBot.BP_TrackerBot_C" (Math|Transform|MakeTransform _array_element) "AdjustIfPossibleButDontSpawnIfColliding" 0 0)))))

(event EventBeginPlay
  (bind _returnvalue (AI|EQS|RunEQSQuery "/Game/BluePrints/EQS_FindSpawnLocation.EQS_FindSpawnLocation" self "RandomBest25Pct"))
  (EventDispatchers|AssignOnQueryFinishedEvent _returnvalue (delegate Custom|OnQueryFinishedEvent_Event_0))
  (Development|PrintString "Query done" true true "(R=0.000000,G=0.660000,B=1.000000,A=1.000000)" 1e+01))

(fn ConstructionScript)