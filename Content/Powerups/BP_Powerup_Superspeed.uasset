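; Superspeed powerup that temporarily makes the activating player move faster.
; On activation it stores the player and sets the CharacterMovementComponent's MaxWalkSpeed to its current max speed multiplied by pi.
; On expiry it divides the current max speed by pi for that player, if still valid, then calls the parent expiry logic.
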(event EventOnActivated
  (params (ActivateFor :type Actor%20Object%20Reference))
  (bind _returnvalue (Actor|GetComponentbyClass ActivateFor "/Script/Engine.CharacterMovementComponent"))
  (Variables|Default|SetActivatedForPlayer ActivateFor)
  (Variables|/Script/Engine.CharacterMovementComponent|SetMaxWalkSpeed _returnvalue (Math|Float|MultiplybyPi (Class|MovementComponent|GetMaxSpeed _returnvalue))))

(event EventOnExpired
  (bind _activatedforplayer (Variables|Default|GetActivatedForPlayer))
  (bind _returnvalue (Actor|GetComponentbyClass _activatedforplayer "/Script/Engine.CharacterMovementComponent"))
  (Utilities|IsValid _activatedforplayer
    (:Is%20Valid
      (Variables|/Script/Engine.CharacterMovementComponent|SetMaxWalkSpeed _returnvalue (/ (Class|MovementComponent|GetMaxSpeed _returnvalue) (Math|Trig|GetPI))))
    (:Is%20Not%20Valid
      _))
  (|CallParentFunction))

(fn ConstructionScript)